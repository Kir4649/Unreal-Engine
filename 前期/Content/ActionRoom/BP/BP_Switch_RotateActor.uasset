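; Switch Blueprint in ActionRoom that drives a quarter-turn yaw rotation when its button is pressed.
; On press, it captures RotateActor's current yaw as the start and adds 90 degrees for the finish.
; The Rotate timeline lerps between them through SetActorRotation, zeroing pitch and roll.
; When the turn finishes, it reverses the ButtonUpDown timeline; button release does nothing here.
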(event EventBeginPlay
  (|CallParentFunction) ; このノードは無効になっているため呼び出せません。\n機能をビルドするにはピンをドラッグしてください。
)

(event Collision|EventActorBeginOverlap
  (params (OtherActor :type Actor%20Object%20Reference))
  (|CallParentFunction OtherActor) ; このノードは無効になっているため呼び出せません。\n機能をビルドするにはピンをドラッグしてください。
)

(event EventTick
  (params (DeltaSeconds :type Float%20%28single-precision%29))
  (|CallParentFunction DeltaSeconds) ; このノードは無効になっているため呼び出せません。\n機能をビルドするにはピンをドラッグしてください。
)

(event EventOnPressedButton
  (bind _rotateactor (Variables|Default|GetRotateActor))
  (bind _returnvalue (Transformation|GetActorRotation _rotateactor))
  (bind _yaw (Math|Rotator|BreakRotator _returnvalue))
  (Variables|Default|SetStartAngle _yaw)
  (Variables|Default|SetFinishAngle (+ _yaw 9e+01))
  (bind _angle (Timeline|Rotate PlayFromStart)
    (:Update
      (Transformation|SetActorRotation (Math|Rotator|MakeRotator 0.0 0.0 (Math|Float|Lerp (Variables|Default|GetStartAngle) (Variables|Default|GetFinishAngle) _angle))))
    (:Finished
      (Components|Timeline|ReversefromEnd (Variables|Default|GetButtonUpDown)))))

(event EventOnReleasedButton)

(fn ConstructionScript
  (|CallParentFunction))