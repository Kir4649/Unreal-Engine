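; Switch Blueprint that rotates a referenced RotateActor when the button's release event fires; the press event is empty.
; OnReleasedButton takes the actor's current yaw and that value plus 90 degrees as endpoints, then plays the Rotate timeline to interpolate between them.
; The interpolated angle is written to roll, with pitch and yaw zeroed.
; When rotation finishes, the ButtonUpDown timeline reverses from its end.
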(event EventBeginPlay
  (|CallParentFunction) ; このノードは無効になっているため呼び出せません。\n機能をビルドするにはピンをドラッグしてください。
)

(event Collision|EventActorBeginOverlap
  (params (OtherActor :type Actor%20Object%20Reference))
  (|CallParentFunction OtherActor) ; このノードは無効になっているため呼び出せません。\n機能をビルドするにはピンをドラッグしてください。
)

(event EventTick
  (params (DeltaSeconds :type Float%20%28single-precision%29))
  (|CallParentFunction DeltaSeconds) ; このノードは無効になっているため呼び出せません。\n機能をビルドするにはピンをドラッグしてください。
)

(event EventOnPressedButton)

(event EventOnReleasedButton
  (bind _rotateactor (Variables|Default|GetRotateActor))
  (bind _output (Utilities|ResolveSoftReference _rotateactor))
  (bind _returnvalue (Transformation|GetActorRotation _output))
  (bind _yaw (Math|Rotator|BreakRotator _returnvalue))
  (Variables|Default|SetStartAngle _yaw)
  (Variables|Default|SetFinishAngle (+ _yaw 9e+01))
  (bind _angle (Timeline|Rotate PlayFromStart)
    (:Update
      (Transformation|SetActorRotation (Utilities|ResolveSoftReference (Variables|Default|GetRotateActor)) (Math|Rotator|MakeRotator (Math|Float|Lerp (Variables|Default|GetStartAngle) (Variables|Default|GetFinishAngle) _angle) 0.0 0.0)))
    (:Finished
      (Components|Timeline|ReversefromEnd (Variables|Default|GetButtonUpDown)))))

(fn ConstructionScript
  (|CallParentFunction))